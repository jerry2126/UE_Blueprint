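; BP_cube is a simple actor Blueprint that slides along world X while spinning around its vertical axis.
; BeginPlay prints the starting location, re-applies it unchanged and resets rotation to zero.
; Tick then adds a fixed step to location and yaw each frame without delta-time scaling or sweep, so speed follows frame rate and movement ignores collision.
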(event EventBeginPlay
  (Development|PrintString (Utilities|String|ToString(Vector) (Transformation|GetActorLocation)) true true "(R=0.000000,G=0.660000,B=1.000000,A=1.000000)" 2e+01)
  (Transformation|SetActorLocation (Transformation|GetActorLocation) false false)
  (Transformation|SetActorRotation "0.000000,0.000000,0.000000"))

(event EventTick
  (params (DeltaSeconds :type Float%20%28single-precision%29))
  (bind _returnvalue (Transformation|GetActorRotation))
  (Transformation|SetActorLocation (+ (Transformation|GetActorLocation) "1.000000,0.000000,0.000000") false false)
  (Transformation|SetActorRotation (Math|Rotator|MakeRotator (.roll _returnvalue) (.pitch _returnvalue) (+ (.yaw _returnvalue) 1.0))))

(fn ConstructionScript)