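; BP_Player is the player-controlled character, handling movement, look and jump through Enhanced Input.
; On BeginPlay it casts its controller to a PlayerController and adds the IMC_Player mapping context.
; IA_Move drives movement along the actor's forward (X) and right (Y) vectors.
; IA_Look feeds controller yaw and pitch, and IA_Jump triggers Jump when started.
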(event Input|EnhancedActionEvents|EnhancedInputActionIA_Jump
  (params (ActionValue :type Boolean) (ElapsedSeconds :type Float%20%28double-precision%29) (TriggeredSeconds :type Float%20%28double-precision%29) (InputAction :type Input%20Action%20Object%20Reference :default "/Game/Blueprints/Inputs/IA_Jump.IA_Jump"))
  (:Started
    (Character|Jump)))

(event Input|EnhancedActionEvents|EnhancedInputActionIA_Look
  (params (ActionValue :type Vector%202D%20Structure) (ElapsedSeconds :type Float%20%28double-precision%29) (TriggeredSeconds :type Float%20%28double-precision%29) (InputAction :type Input%20Action%20Object%20Reference :default "/Game/Blueprints/Inputs/IA_Look.IA_Look"))
  (:Triggered
    (Pawn|Input|AddControllerYawInput (.x ActionValue)) ; Add Controller(카메라)에 적용하라\n마우스는 좌표계가 다름(스크린좌표계)\nX축값을 받아서 Z축으로 회전하도록 변환하는중(Yaw=Z)\n짐벌락 기능을 막기위해 사용\n주로 시야기능에 사용\n캐릭터에 입력을 주는것이 아닌  카메라에 입력 중
    (Pawn|Input|AddControllerPitchInput (.y ActionValue))))

(event Input|EnhancedActionEvents|EnhancedInputActionIA_Move
  (params (ActionValue :type Vector%202D%20Structure) (ElapsedSeconds :type Float%20%28double-precision%29) (TriggeredSeconds :type Float%20%28double-precision%29) (InputAction :type Input%20Action%20Object%20Reference :default "/Game/Blueprints/Inputs/IA_Move.IA_Move"))
  (Pawn|Input|AddMovementInput (Transformation|GetActorForwardVector) (.x ActionValue) false)
  (Pawn|Input|AddMovementInput (Transformation|GetActorRightVector) (.y ActionValue) false))

(event EventBeginPlay
  (bind _as플레이어_컨트롤러 (Utilities|Casting|CastToPlayerController (Pawn|GetController)))
  (Input|AddMappingContext (PlayerController|LocalPlayerSubsystems|GetEnhancedInputLocalPlayerSubsystem _as플레이어_컨트롤러) "/Game/Blueprints/Inputs/IMC_Player.IMC_Player" 0 "(bIgnoreAllPressedKeysUntilRelease=True,bForceImmediately=False,bNotifyUserSettings=False)"))

(fn ConstructionScript)