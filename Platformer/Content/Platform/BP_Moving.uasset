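; BP_Moving is a platform actor whose mesh travels toward an ArrivalPoint component.
; BeginPlay hides the ArrivalPoint in game.
; Each Tick shifts PlatformMesh by the normalized direction to that point, without sweep.
; The one-unit step per frame is not scaled by DeltaSeconds, so speed depends on frame rate, and no arrival check exists.
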(event EventBeginPlay
  (|CallParentFunction)
  (Development|SetHiddeninGame (Variables|Default|GetArrivalPoint) true false) ; 겜임 플레이시 렌더링 안함\nNew hidden 체크
)

(event EventTick
  (params (DeltaSeconds :type Float%20%28single-precision%29))
  (bind _platformmesh (Variables|Default|GetPlatformMesh))
  (bind _returnvalue (Transformation|GetWorldLocation _platformmesh))
  (|CallParentFunction DeltaSeconds)
  (Transformation|SetWorldLocation _platformmesh (+ _returnvalue (Math|Vector|Normalize (- (Transformation|GetWorldLocation (Variables|Default|GetArrivalPoint)) _returnvalue))) false false))

(fn ConstructionScript
  (|CallParentFunction))